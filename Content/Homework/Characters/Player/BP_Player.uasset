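; Player character Blueprint, apparently a homework test bed for two toggleable invisibility effects on the mesh.
; Keys 1 and 2 create dynamic material instances on both mesh slots, then play or reverse timelines driving dithered opacity or refractive fill amount.
; Tick positions two spheres at the left and right foot IK offsets.
; Sprint events only call the parent; the spring-arm length timeline is never triggered.
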(event `self.ReceiveTick`
  (params (DeltaSeconds :type "Float (single-precision)"))
  ;[1 1 1] Leg IK Location
  (`SceneComponent.K2_SetRelativeLocation` (`self.Sphere`) (`KismetMathLibrary.MakeVector` 0.0 200.0 (`self.GetIKRightFootOffset`)) false false)
  (`SceneComponent.K2_SetRelativeLocation` (`self.Sphere1`) (`KismetMathLibrary.MakeVector` 0.0 150.0 (`self.GetIKLeftFootOffset`)) false false))

(event `Key|Two`
  (params (Key :type "Key Structure"))
  (bind _mesh (`self.Mesh`))
  ;[1 1 1] Filling Refractive Invisibility
  (:`Pressed`
    (`|ExecutionSequence`
      (:`then_0`
        (bind _returnvalue (`PrimitiveComponent.CreateDynamicMaterialInstance` _mesh 0 "/Game/Homework/Characters/Player/Materials/MI_Invisibility_Filling_Inst.MI_Invisibility_Filling_Inst" "None"))
        (set `self.Filling Invis DMaterial` _returnvalue)
        (`/Engine/EditorBlueprintResources/StandardMacros.FlipFlop`
          (:`A`
            (`KismetSystemLibrary.PrintString` "Refraction Invisibility On")
            (bind (_direction _newtrack_0) (`Timeline|Timeline_0` :!label _label)
              (:`Update`
                (`MaterialInstanceDynamic.SetScalarParameterValue` (`self.Filling Invis DMaterial`) "Amount" _newtrack_0)
                (`MaterialInstanceDynamic.SetScalarParameterValue` (`self.Filling Invis DMaterial 2`) "Amount" _newtrack_0))))
          (:`B`
            (`KismetSystemLibrary.PrintString` "Refraction Invisibility Off")
            (goto _label :!via `Reverse`))))
      (:`then_1`
        (bind _returnvalue_2 (`PrimitiveComponent.CreateDynamicMaterialInstance` _mesh 1 "/Game/Homework/Characters/Player/Materials/MI_Invisibility_Filling_Inst.MI_Invisibility_Filling_Inst" "None"))
        (set `self.Filling Invis DMaterial 2` _returnvalue_2)))))

(event `self.OnSprintStart`
  (`parent.OnSprintStart`))

(event `self.OnSprintEnd`
  (`parent.OnSprintEnd`))

(event `self.ReceiveBeginPlay`
  ;[1 1 1] Spring Arm
  (set `self.DefaultArmLength_0` (`SpringArmComponent.TargetArmLength` (`self.SpringArmComponent`))))

(event `Key|One`
  (params (Key :type "Key Structure"))
  (bind _mesh (`self.Mesh`))
  ;[1 1 1] Temporal Tithering Invisibility
  (:`Pressed`
    (`|ExecutionSequence`
      (:`then_0`
        (bind _returnvalue (`PrimitiveComponent.CreateDynamicMaterialInstance` _mesh 0 "/Game/Homework/Characters/Player/Materials/M_Male_Body.M_Male_Body" "None"))
        (set `self.DMaterial` _returnvalue)
        (`/Engine/EditorBlueprintResources/StandardMacros.FlipFlop`
          (:`A`
            (`KismetSystemLibrary.PrintString` "Dithering Invisibility On")
            (bind (_direction _newtrack_0) (`Timeline|Invisible` :!label _label_2)
              (:`Update`
                (`MaterialInstanceDynamic.SetScalarParameterValue` (`self.DMaterial`) "Opacity" _newtrack_0)
                (`MaterialInstanceDynamic.SetScalarParameterValue` (`self.DMaterial 2`) "Opacity" _newtrack_0))))
          (:`B`
            (`KismetSystemLibrary.PrintString` "Dithering Invisiblility Off")
            (goto _label_2 :!via `Reverse`))))
      (:`then_1`
        (bind _returnvalue_2 (`PrimitiveComponent.CreateDynamicMaterialInstance` _mesh 1 "/Game/Homework/Characters/Player/Materials/M_UE4Man_ChestLogo.M_UE4Man_ChestLogo" "None"))
        (set `self.DMaterial 2` _returnvalue_2)))))

(fn `UserConstructionScript`)